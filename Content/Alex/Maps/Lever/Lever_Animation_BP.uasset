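; Lever socket actor that lets a player carrying the matching lever place it and open a linked door.
; Box overlap checks the FirstPersonCharacter's Lever array at the LeverValue index, then enables input and flags the player in range, with no reset on exit.
; Pressing E shows the lever mesh, plays its animation, opens TargetDoor and removes a lever from the player once via DoOnce.
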(event `Lever_Intact`
  (`SkeletalMeshComponent.PlayAnimation` (`self.Lever`) "/Game/Alex/Maps/Lever/Lever_Animation_pCylinder5_Anim.Lever_Animation_pCylinder5_Anim" false)
  (set `self.Lever_Open` true))

(event `Place_lever`
  (`SceneComponent.SetVisibility` (`self.Lever`) true false)
  (set `self.Has_Lever` true))

(event `self.Box.OnComponentBeginOverlap`
  (params (OverlappedComponent :type "PrimitiveComponent Object Reference") (OtherActor :type "Actor Object Reference") (OtherComp :type "PrimitiveComponent Object Reference") (OtherBodyIndex :type Integer) (bFromSweep :type Boolean) (SweepResult :type "HitResult Structure (by ref)"))
  (bind _asfirst_person_character (cast `/Game/FirstPersonBP/Blueprints/FirstPersonCharacter` OtherActor))
  (for (_array_element _array_index) (`/Game/FirstPersonBP/Blueprints/FirstPersonCharacter.Lever` _asfirst_person_character)
    (if (and _array_element (== _array_index (`self.Lever Value`)))
      (set `self.Player_In_Range` true)
      (`self.EnableInput` (`GameplayStatics.GetPlayerController` 0)))))

(event `Key|E`
  (params (Key :type "Key Structure"))
  (:`Pressed`
    (if (`self.Player_In_Range`)
      (`SceneComponent.SetVisibility` (`self.Lever`) true false)
      (`self.Lever_Intact`)
      (`/Game/Alex/Maps/Door_Lever.Door Open` (`self.Target Door`))
      ;[1 1 1] remove 1 lever once from lever_amount(player inventory)
      (bind _asfirst_person_character (cast `/Game/FirstPersonBP/Blueprints/FirstPersonCharacter` (stale `self.Box.OnComponentBeginOverlap` _asfirst_person_character)))
      (`/Engine/EditorBlueprintResources/StandardMacros.DoOnce` false
        (:`Completed`
          (`/Game/FirstPersonBP/Blueprints/FirstPersonCharacter.remove_lever` _asfirst_person_character))))))

(fn `UserConstructionScript`)