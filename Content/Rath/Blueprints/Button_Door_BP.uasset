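; Four-button puzzle door: the player must press the randomly chosen star button to move the door, while a wrong press pauses the game on a retry/game-over widget.
; BeginPlay picks the correct index and assigns the star and remaining materials.
; Overlap volumes set the current button index, and Interact plays that button's press timeline before checking the answer.
; A FlipFlop plays or reverses the door timeline on each correct press.
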(event `self.ReceiveBeginPlay`
  (bind _material (`self.material`))
  ;[1 1 1] Shuffle button order at the start
  (set `self.buttons` (`|MakeArray` (`self.button_1`) (`self.button_2`) (`self.button_3`) (`self.button_4`)))
  (set `self.correct_button_index` (`KismetMathLibrary.RandomIntegerInRange` 0 3))
  (`self.EnableInput` (`GameplayStatics.GetPlayerController` 0))
  (for (_array_element _array_index) (`self.buttons`)
    (if (== _array_index (`self.correct_button_index`))
      (`PrimitiveComponent.SetMaterial` _array_element 0 "/Game/Rath/Materials/button_star.button_star")
      (else
        (`PrimitiveComponent.SetMaterial` _array_element 0 (`|GetArrayItem` _material))
        (`KismetArrayLibrary.Array_Remove` _material)))))

(event `self.interaction_2.OnComponentBeginOverlap`
  (params (OverlappedComponent :type "PrimitiveComponent Object Reference") (OtherActor :type "Actor Object Reference") (OtherComp :type "PrimitiveComponent Object Reference") (OtherBodyIndex :type Integer) (bFromSweep :type Boolean) (SweepResult :type "HitResult Structure (by ref)"))
  ;[1 1 1] Set button 1 index, press E to interact if within collider box
  (set `self.current_button_index` 1)
  (cast `/Game/FirstPersonBP/Blueprints/FirstPersonCharacter` OtherActor)
  (set `self.in_button_range` true))

(event `self.interaction_2.OnComponentEndOverlap`
  (params (OverlappedComponent :type "PrimitiveComponent Object Reference") (OtherActor :type "Actor Object Reference") (OtherComp :type "PrimitiveComponent Object Reference") (OtherBodyIndex :type Integer))
  ;[1 1 1] Set button 1 index, press E to interact if within collider box
  (cast `/Game/FirstPersonBP/Blueprints/FirstPersonCharacter` OtherActor)
  (set `self.in_button_range` false))

(event `correctButton`
  ;[1 1 1] Door move anim & coord
  (`AddComponent|NODE_AddAudioComponent-1`)
  (`/Engine/EditorBlueprintResources/StandardMacros.FlipFlop`
    (:`A`
      (bind (_direction _door_track) (`Timeline|Timeline_2` :!label _label)
        (:`Update`
          (`SceneComponent.K2_SetRelativeLocation` (`self.Door`) (`KismetMathLibrary.VLerp` (`self.A`) (`self.B`) _door_track) false false))))
    (:`B`
      (goto _label :!via `Reverse`))))

(event `InputAction|Interact`
  (params (Key :type "Key Structure"))
  (:`Pressed`
    (if (`self.in_button_range`)
      (switch `int` (`self.current_button_index`)
        (:`0`
          (bind (_direction _button_track) (`Timeline|Timeline_6` :!via `PlayFromStart`)
            (:`Update`
              (`SceneComponent.K2_SetRelativeLocation` (`self.button_1`) (`KismetMathLibrary.VLerp` (-330.0 80.0 150.0) (-330.0 70.0 150.0) _button_track) false false))
            (:`Finished`
              (`AddComponent|NODE_AddAudioComponent-3` :!label _label_2)
              ;[1 1 1] Check if player presses the correct button or not
              (if (== (`self.current_button_index`) (`self.correct_button_index`))
                (`self.correctButton`)
                (else
                  (`self.incorrectButton`))))))
        (:`1`
          (bind (_direction_2 _button_track_2) (`Timeline|Timeline_1` :!via `PlayFromStart`)
            (:`Update`
              (`SceneComponent.K2_SetRelativeLocation` (`self.button_2`) (`KismetMathLibrary.VLerp` (-230.0 80.0 150.0) (-230.0 70.0 150.0) _button_track_2) false false))
            (:`Finished`
              (goto _label_2))))
        (:`2`
          (bind (_direction_3 _button_track_3) (`Timeline|Timeline_3` :!via `PlayFromStart`)
            (:`Update`
              (`SceneComponent.K2_SetRelativeLocation` (`self.button_3`) (`KismetMathLibrary.VLerp` (80.0 80.0 150.0) (80.0 70.0 150.0) _button_track_3) false false))
            (:`Finished`
              (goto _label_2))))
        (:`3`
          (bind (_direction_4 _button_track_4) (`Timeline|Timeline_4` :!via `PlayFromStart`)
            (:`Update`
              (`SceneComponent.K2_SetRelativeLocation` (`self.button_4`) (`KismetMathLibrary.VLerp` (170.0 80.0 150.0) (170.0 70.0 150.0) _button_track_4) false false))
            (:`Finished`
              (goto _label_2))))))))

(event `self.interaction_3.OnComponentBeginOverlap`
  (params (OverlappedComponent :type "PrimitiveComponent Object Reference") (OtherActor :type "Actor Object Reference") (OtherComp :type "PrimitiveComponent Object Reference") (OtherBodyIndex :type Integer) (bFromSweep :type Boolean) (SweepResult :type "HitResult Structure (by ref)"))
  ;[1 1 1] Set button 2 index, press E to interact if within collider box
  (set `self.current_button_index` 2)
  (cast `/Game/FirstPersonBP/Blueprints/FirstPersonCharacter` OtherActor)
  (set `self.in_button_range` true))

(event `self.interaction_3.OnComponentEndOverlap`
  (params (OverlappedComponent :type "PrimitiveComponent Object Reference") (OtherActor :type "Actor Object Reference") (OtherComp :type "PrimitiveComponent Object Reference") (OtherBodyIndex :type Integer))
  ;[1 1 1] Set button 2 index, press E to interact if within collider box
  (cast `/Game/FirstPersonBP/Blueprints/FirstPersonCharacter` OtherActor)
  (set `self.in_button_range` false))

(event `incorrectButton`
  ;[1 1 1] Send player to lose screen
  (bind _returnvalue (`|CreateWidget` "/Game/Emma/BluePrints/Retry_GameOver.Retry_GameOver_C" (`GameplayStatics.GetPlayerController` 0)))
  (`UserWidget.AddToViewport` _returnvalue 0)
  (set `PlayerController.bShowMouseCursor` true (`GameplayStatics.GetPlayerController` 0))
  (`GameplayStatics.SetGamePaused` true))

(event `self.interaction_4.OnComponentBeginOverlap`
  (params (OverlappedComponent :type "PrimitiveComponent Object Reference") (OtherActor :type "Actor Object Reference") (OtherComp :type "PrimitiveComponent Object Reference") (OtherBodyIndex :type Integer) (bFromSweep :type Boolean) (SweepResult :type "HitResult Structure (by ref)"))
  ;[1 1 1] Set button 3 index, press E to interact if within collider box
  (set `self.current_button_index` 3)
  (cast `/Game/FirstPersonBP/Blueprints/FirstPersonCharacter` OtherActor)
  (set `self.in_button_range` true))

(event `self.interaction_4.OnComponentEndOverlap`
  (params (OverlappedComponent :type "PrimitiveComponent Object Reference") (OtherActor :type "Actor Object Reference") (OtherComp :type "PrimitiveComponent Object Reference") (OtherBodyIndex :type Integer))
  ;[1 1 1] Set button 3 index, press E to interact if within collider box
  (cast `/Game/FirstPersonBP/Blueprints/FirstPersonCharacter` OtherActor)
  (set `self.in_button_range` false))

(event `self.interaction_1.OnComponentBeginOverlap`
  (params (OverlappedComponent :type "PrimitiveComponent Object Reference") (OtherActor :type "Actor Object Reference") (OtherComp :type "PrimitiveComponent Object Reference") (OtherBodyIndex :type Integer) (bFromSweep :type Boolean) (SweepResult :type "HitResult Structure (by ref)"))
  ;[1 1 1] Set button 4 index, press E to interact if within collider bo
  (set `self.current_button_index` 0)
  (cast `/Game/FirstPersonBP/Blueprints/FirstPersonCharacter` OtherActor)
  (set `self.in_button_range` true))

(event `self.interaction_1.OnComponentEndOverlap`
  (params (OverlappedComponent :type "PrimitiveComponent Object Reference") (OtherActor :type "Actor Object Reference") (OtherComp :type "PrimitiveComponent Object Reference") (OtherBodyIndex :type Integer))
  ;[1 1 1] Set button 4 index, press E to interact if within collider bo
  (cast `/Game/FirstPersonBP/Blueprints/FirstPersonCharacter` OtherActor)
  (set `self.in_button_range` false))

(fn `UserConstructionScript`)